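; BP_ZoneCheck detects which kind of tagged decal zone it touches and records it in a DecalType enum.
; On Box begin overlap, it reads the other component's Decal and PinkDecal tags to pick pink decal, other decal or no decal.
; An older downward line trace from an Arrow, doing the same classification, remains disconnected, and the Raycast event is empty.
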(event OnComponentBeginOverlap(Box)
  (params (OverlappedComponent :type Primitive%20Component%20Object%20Reference) (OtherActor :type Actor%20Object%20Reference) (OtherComp :type Primitive%20Component%20Object%20Reference) (OtherBodyIndex :type Integer) (bFromSweep :type Boolean) (SweepResult :type Hit%20Result%20Structure%20%28by%20ref%29))
  (if (Components|ComponentHasTag OtherComp "Decal")
    (if (Components|ComponentHasTag OtherComp "PinkDecal")
      (Variables|Default|SetdecalType "NewEnumerator1")
      (else
        (Variables|Default|SetdecalType "NewEnumerator2")))
    (else
      (Variables|Default|SetdecalType "NewEnumerator0"))))

(event Custom|Raycast)

(fn ConstructionScript)