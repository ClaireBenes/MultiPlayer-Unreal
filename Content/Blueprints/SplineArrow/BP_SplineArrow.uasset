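; BP_SplineArrow is an actor that draws an arrow along an editable spline, built entirely in the construction script.
; It adds a spline mesh for each segment between neighboring points, fitted to their local positions and tangents with X as the forward axis.
; Each segment gets a uniform cross-section scale and a dynamic M_Arrow material driven by the color, glow and speed variables.
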(event EventBeginPlay)

(event Collision|EventActorBeginOverlap
  (params (OtherActor :type Actor%20Object%20Reference)))

(event EventTick
  (params (DeltaSeconds :type Float%20%28single-precision%29)))

(fn ConstructionScript
  (for _index (range 0 (- (Spline|GetNumberOfSplinePoints (Variables|Default|GetSpline)) 2))
    (bind _returnvalue (AddComponent|AddSplineMeshComponent false))
    (Variables|Default|SetAs%20Spline%20Mesh _returnvalue)
    (CallFunction|SetScale)
    (CallFunction|AdjustArrowParameters)
    (SplineMesh|SetForwardAxis (Variables|Default|GetAs%20Spline%20Mesh) "X" true)
    (SplineMesh|SetStartandEnd (Variables|Default|GetAs%20Spline%20Mesh) (.StartPos (Utilities|GetStartandEndPos _index (+ _index 1))) (.StartTangent (Utilities|GetStartandEndPos _index (+ _index 1))) (.EndPos (Utilities|GetStartandEndPos _index (+ _index 1))) (.EndTangent (Utilities|GetStartandEndPos _index (+ _index 1))) true :!class /Script/Engine.SplineMeshComponent)))

(fn AdjustArrowParameters
  (bind _returnvalue (Rendering|Material|CreateDynamicMaterialInstance (Variables|Default|GetAs%20Spline%20Mesh) 0 "/Game/Blueprints/SplineArrow/M_Arrow.M_Arrow" "None" :!class /Script/Engine.PrimitiveComponent))
  (Rendering|Material|SetVectorParameterValue _returnvalue "Color" (Variables|Default|GetColor) :!class /Script/Engine.MaterialInstanceDynamic)
  (Rendering|Material|SetScalarParameterValue _returnvalue "Glow" (Variables|Default|GetGlow) :!class /Script/Engine.MaterialInstanceDynamic)
  (Rendering|Material|SetScalarParameterValue _returnvalue "Speed" (Variables|Default|GetSpeed) :!class /Script/Engine.MaterialInstanceDynamic))

(fn SetScale
  (bind _scale (Variables|Default|GetScale))
  (bind _as_spline_mesh (Variables|Default|GetAs%20Spline%20Mesh))
  (bind _returnvalue (Math|Vector2D|MakeVector2D _scale _scale))
  (SplineMesh|SetStartScale _as_spline_mesh _returnvalue true :!class /Script/Engine.SplineMeshComponent)
  (SplineMesh|SetEndScale _as_spline_mesh _returnvalue true :!class /Script/Engine.SplineMeshComponent))