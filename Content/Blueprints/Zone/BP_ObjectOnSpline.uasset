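; Zone actor, such as a column, that travels along a referenced BPSpline once the game starts.
; BeginPlay snaps it to the spline's first point and registers a start event with the GS_GameMap game state.
; The move event plays a timeline at a rate of 1/TimeToComplete, mapping its track to distance along the spline.
; Only X and Y follow the spline, while the actor keeps its own height.
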(event Custom|M_Move
  ;[1 1 1] Movement on Spline
  (Components|Timeline|SetPlayRate (Variables|Default|GetMoveObject) (/ 1.0 (Variables|Default|GettimeToComplete)))
  (bind _movetrack (Timeline|MoveObject Play)
    (:Update
      (Transformation|SetActorTransform (Math|Transform|MakeTransform (Math|Vector|MakeVector (.x (Spline|GetLocationatDistanceAlongSpline (Variables|/Game/Blueprints/Zone/BP_SplineZone.BP_SplineZone_C|GetSpline (Variables|Default|GetAs%20BP%20Spline)) (Math|Float|Lerp 0.0 (Spline|GetSplineLength (Variables|/Game/Blueprints/Zone/BP_SplineZone.BP_SplineZone_C|GetSpline (Variables|Default|GetAs%20BP%20Spline))) _movetrack) "World")) (.y (Spline|GetLocationatDistanceAlongSpline (Variables|/Game/Blueprints/Zone/BP_SplineZone.BP_SplineZone_C|GetSpline (Variables|Default|GetAs%20BP%20Spline)) (Math|Float|Lerp 0.0 (Spline|GetSplineLength (Variables|/Game/Blueprints/Zone/BP_SplineZone.BP_SplineZone_C|GetSpline (Variables|Default|GetAs%20BP%20Spline))) _movetrack) "World")) (.z (Transformation|GetActorLocation))) "0, 0, 0" "1.000000,1.000000,1.000000")))))

(event Custom|gameStart_Event
  ;[1 1 1] Begin Play
  ;;[1 0.2986 0.3019] Moving Column
  (CallFunction|MMove))

(event EventBeginPlay
  (bind _as_bp_spline (Variables|Default|GetAs%20BP%20Spline))
  (bind _spline (Variables|/Game/Blueprints/Zone/BP_SplineZone.BP_SplineZone_C|GetSpline _as_bp_spline))
  (bind _returnvalue (Spline|GetTransformatSplinePoint _spline 0 "World" false))
  ;[1 1 1] Begin Play
  ;;[0.7523 1 0.531] PutColumnAtRightPos
  (Transformation|SetActorTransform (Math|Transform|MakeTransform (Math|Vector|MakeVector (.x (.location _returnvalue)) (.y (.location _returnvalue)) (.z (Transformation|GetActorLocation))) "0, 0, 0" "1.000000,1.000000,1.000000"))
  ;;[1 0.2986 0.3019] Moving Column
  (EventDispatchers|AssignGameStart (.AsGS%20Game%20Map (Utilities|Casting|CastToGS_GameMap (Game|GetGameState))) (delegate Custom|gameStart_Event)))

(fn ConstructionScript)