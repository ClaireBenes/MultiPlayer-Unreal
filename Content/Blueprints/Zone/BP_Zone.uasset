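; Capturable zone that pink and green teams fight to control by covering it with paint decals.
; On BeginPlay it spawns a grid of BP_ZoneCheck points from the box bounds, then tallies their colors on each box overlap.
; Reaching the win percentage fills all points, clears decals, recolors floor and goal, and notifies GS_GameMap.
; The owner keeps control down to 50% coverage; otherwise, without a new winner, the goal turns neutral.
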(event OnComponentBeginOverlap(Box)
  (params (OverlappedComponent :type Primitive%20Component%20Object%20Reference) (OtherActor :type Actor%20Object%20Reference) (OtherComp :type Primitive%20Component%20Object%20Reference) (OtherBodyIndex :type Integer) (bFromSweep :type Boolean) (SweepResult :type Hit%20Result%20Structure%20%28by%20ref%29))
  ;[1 1 1] Check whole zone everytime someone fire in the zone
  (if (Actor|ActorHasTag OtherActor "Decal")
    (Utilities|Array|Add (Variables|Default|GetallDecals) (.AsBP%20Decal (Utilities|Casting|CastToBP_Decal OtherActor))))
  (Variables|Zone|Control|SetpinkZones 0)
  (Variables|Zone|Control|SetgreenZones 0)
  (for _array_element (Variables|Default|GetzoneCheck)
    (if (Utilities|Enum|Equal(Enum) (Variables|/Game/Blueprints/Zone/BP_ZoneCheck.BP_ZoneCheck_C|GetdecalType _array_element) "NewEnumerator1")
      (Variables|Zone|Control|SetpinkZones (+ (Variables|Zone|Control|GetpinkZones) 1))
      (elif (Utilities|Enum|Equal(Enum) (Variables|/Game/Blueprints/Zone/BP_ZoneCheck.BP_ZoneCheck_C|GetdecalType _array_element) "NewEnumerator2")
        (Variables|Zone|Control|SetgreenZones (+ (Variables|Zone|Control|GetgreenZones) 1)))))
  ;[1 0.1136 0.7714] Pink
  (bind _returnvalue (CallFunction|CheckColorPourcentage (Variables|Zone|Control|GetpinkZones) 5e+01))
  (if (and (Variables|Zone|Control|GetpinkInControl) _returnvalue)
    (Variables|Zone|Control|SetgreenInControl false :!label _label)
    (Variables|Zone|Control|SetpinkInControl true)
    (else
      (bind _returnvalue_2 (CallFunction|CheckColorPourcentage (Variables|Zone|Control|GetpinkZones) (Variables|Zone|Control|Pourcentage|GetwinPourcentage)))
      (if _returnvalue_2
        (for _array_element_2 (Variables|Default|GetzoneCheck)
          (Variables|/Game/Blueprints/Zone/BP_ZoneCheck.BP_ZoneCheck_C|SetdecalType _array_element_2 "NewEnumerator1"))
        (CallFunction|DestroyAllDecals)
        (CallFunction|UpdateFloor "/Game/Material/PaintSplat/MaterialInstance/MI_PinkFloor.MI_PinkFloor" "/Game/Material/MI_PinkGoal.MI_PinkGoal")
        (Default|OCUpdatePourcentage (.AsGS%20Game%20Map (Utilities|Casting|CastToGS_GameMap (Game|GetGameState))) "NewEnumerator1")
        (goto _label)
        (else
          ;[0.2833 1 0.4085] Green
          (bind _returnvalue_3 (CallFunction|CheckColorPourcentage (Variables|Zone|Control|GetgreenZones) 5e+01))
          (if (and (Variables|Zone|Control|GetgreenInControl) _returnvalue_3)
            (Variables|Zone|Control|SetpinkInControl false :!label _label_2)
            (Variables|Zone|Control|SetgreenInControl true)
            (else
              (bind _returnvalue_4 (CallFunction|CheckColorPourcentage (Variables|Zone|Control|GetgreenZones) (Variables|Zone|Control|Pourcentage|GetwinPourcentage)))
              (if _returnvalue_4
                (for _array_element_3 (Variables|Default|GetzoneCheck)
                  (Variables|/Game/Blueprints/Zone/BP_ZoneCheck.BP_ZoneCheck_C|SetdecalType _array_element_3 "NewEnumerator2"))
                (CallFunction|DestroyAllDecals)
                (CallFunction|UpdateFloor "/Game/Material/PaintSplat/MaterialInstance/MI_GreenFloor.MI_GreenFloor" "/Game/Material/MI_GreenGoal.MI_GreenGoal")
                (Default|OCUpdatePourcentage (.AsGS%20Game%20Map (Utilities|Casting|CastToGS_GameMap (Game|GetGameState))) "NewEnumerator2")
                (goto _label_2)
                (else
                  ;[1 1 1] Nobody In Control
                  (Variables|Zone|Control|SetgreenInControl false)
                  (Variables|Zone|Control|SetpinkInControl false)
                  (Rendering|Material|SetMaterial (Variables|Default|GetGoalPoint) 0 "/Game/Material/MI_NoControlGoal.MI_NoControlGoal")
                  (Default|OCUpdatePourcentage (.AsGS%20Game%20Map (Utilities|Casting|CastToGS_GameMap (Game|GetGameState))) "NewEnumerator0"))))))))))

(event EventBeginPlay
  (bind _box (Variables|Default|GetBox))
  (bind _cube (Variables|Default|GetCube))
  (bind _returnvalue (Transformation|GetWorldLocation _cube))
  (bind _boxextent (Collision|GetComponentBounds _box))
  (bind (_x _y) (Math|Vector|BreakVector _boxextent))
  ;[1 1 1] Begin Play
  (Rendering|SetVisibility (Variables|Default|GetFloor) false false)
  ;;[1 0.2846 0.1882] Create Point grid for zone check
  (Variables|Zone|Point|SetrowPos (.x _returnvalue))
  (Variables|Zone|Point|SetcolumnPos (.y _returnvalue))
  (Variables|Zone|SetRow (* (Math|Float|Truncate (/ _x (Variables|Zone|Point|GetoffsetBetweenPoints))) 2))
  (Variables|Zone|SetColumn (* (Math|Float|Truncate (/ _y (Variables|Zone|Point|GetoffsetBetweenPoints))) 2))
  (for _index (range 0 (+ (Variables|Zone|GetRow) 1))
    (for _index_2 (range 0 (Variables|Zone|GetColumn))
      (bind _returnvalue_2 (Game|SpawnActorfromClass "/Game/Blueprints/Zone/BP_ZoneCheck.BP_ZoneCheck_C" (Math|Transform|MakeTransform (Math|Vector|MakeVector (+ (Variables|Zone|Point|GetrowPos) (* _index (Variables|Zone|Point|GetoffsetBetweenPoints))) (+ (* _index_2 (Variables|Zone|Point|GetoffsetBetweenPoints)) (Variables|Zone|Point|GetcolumnPos)) (.z (Transformation|GetActorLocation))) "0, 0, 0" "1.000000,1.000000,1.000000") "Undefined" "MultiplyWithRoot" 0 0))
      (Utilities|Array|Add (Variables|Default|GetzoneCheck) _returnvalue_2))))

(fn ConstructionScript)

(fn CheckColorPourcentage
  (params (zoneNumbers :type Integer) (pourcentage :type Float%20%28double-precision%29))
  (return (>= (* (/ (Math|Conversions|ToFloat(Integer) zoneNumbers) (Math|Conversions|ToFloat(Integer) (Utilities|Array|Length (Variables|Default|GetzoneCheck)))) 1e+02) pourcentage)))

(fn DestroyAllDecals
  (bind _alldecals (Variables|Default|GetallDecals))
  (for _array_element _alldecals
    (Utilities|IsValid _array_element
      (:Is%20Valid
        (Default|Destroying _array_element))))
  (Utilities|Array|Clear _alldecals))

(fn UpdateFloor
  (params (Floor :type Material%20Interface%20Object%20Reference) (Goal :type Material%20Interface%20Object%20Reference))
  (Utilities|FlowControl|Sequence
    (:then_0
      (Utilities|FlowControl|DoOnce false
        (:Completed
          (Rendering|SetVisibility (Variables|Default|GetFloor) true false))))
    (:then_1
      (Rendering|Material|SetMaterial (Variables|Default|GetFloor) 0 Floor)
      (Rendering|Material|SetMaterial (Variables|Default|GetGoalPoint) 0 Goal))))