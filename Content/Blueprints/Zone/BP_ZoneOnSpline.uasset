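; BP_ZoneOnSpline is an actor that travels along the spline of the BP_SplineZone found in the level at BeginPlay.
; M_Move plays a timeline, rate-scaled by TimeToComplete, that maps its track to spline distance and sets the actor's location and rotation.
; A BP_ThirdPersonCharacter entering its Box calls SRMovePlatform on that character; this file does not itself call M_Move.
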(event OnComponentBeginOverlap(Box)
  (params (OverlappedComponent :type Primitive%20Component%20Object%20Reference) (OtherActor :type Actor%20Object%20Reference) (OtherComp :type Primitive%20Component%20Object%20Reference) (OtherBodyIndex :type Integer) (bFromSweep :type Boolean) (SweepResult :type Hit%20Result%20Structure%20%28by%20ref%29))
  (bind _asbp_third_person_character (Utilities|Casting|CastToBP_ThirdPersonCharacter OtherActor))
  (Default|SRMovePlatform _asbp_third_person_character))

(event Custom|M_Move
  (bind _as_bp_spline (Variables|Default|GetAs%20BP%20Spline))
  (bind _spline (Variables|/Game/Blueprints/Zone/BP_SplineZone.BP_SplineZone_C|GetSpline _as_bp_spline))
  (Components|Timeline|SetPlayRate (Variables|Default|GetMoveObject) (/ 1.0 (Variables|Default|GettimeToComplete)))
  (bind _movetrack (Timeline|MoveObject Play)
    (:Update
      (Transformation|SetActorTransform (Math|Transform|MakeTransform (Spline|GetLocationatDistanceAlongSpline _spline (Math|Float|Lerp 0.0 (Spline|GetSplineLength (Variables|/Game/Blueprints/Zone/BP_SplineZone.BP_SplineZone_C|GetSpline (Variables|Default|GetAs%20BP%20Spline))) _movetrack) "World") (Spline|GetRotationatDistanceAlongSpline _spline (Math|Float|Lerp 0.0 (Spline|GetSplineLength (Variables|/Game/Blueprints/Zone/BP_SplineZone.BP_SplineZone_C|GetSpline (Variables|Default|GetAs%20BP%20Spline))) _movetrack) "World") "1.000000,1.000000,1.000000")))))

(event EventBeginPlay
  (bind _returnvalue (Actor|GetActorOfClass "/Game/Blueprints/Zone/BP_SplineZone.BP_SplineZone_C"))
  (Variables|Default|SetAs%20BP%20Spline _returnvalue))

(fn ConstructionScript)