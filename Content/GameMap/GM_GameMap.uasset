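; Game mode for the game map that spawns and respawns players at Pink or Green team player starts.
; On login it saves through GI_Framework, sorts tagged starts once, then spawns and possesses a BP_ThirdPersonCharacter.
; Team comes from the decal class in PS_Lobby; respawn teleports the existing character instead of creating another.
; Both paths cycle through starts round-robin using one index shared by both teams.
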(event Custom|Respawn
  (params (actorToRespawn :type BP%20Third%20Person%20Character%20Object%20Reference))
  (bind _output_get (Variables|Default|Setplayer%20to%20Respawn actorToRespawn))
  (if (== (Variables|/Game/Lobby/PS_Lobby.PS_Lobby_C|GetPBDecalClass (.AsPS%20Lobby (Utilities|Casting|CastToPS_Lobby (Variables|/Script/Engine.Controller|GetPlayerState (Pawn|GetController _output_get))))) "/Game/Blueprints/Decal/BP_DecalPink.BP_DecalPink_C")
    (CallFunction|RespawnPlayer (Variables|Default|GetpinkPlayerStarts))
    (else
      (CallFunction|RespawnPlayer (Variables|Default|GetgreenPlayerStarts)))))

(event EventPostLogin
  (params (NewPlayer :type Player%20Controller%20Object%20Reference))
  ;[1 1 1] Spawn Actor at corresponding player start
  (bind _output_get (Variables|Default|SetnewPlayer NewPlayer))
  (bind _asgi_framework (Utilities|Casting|CastToGI_Framework (Game|GetGameInstance)))
  (Default|SaveGame _asgi_framework)
  (Utilities|FlowControl|Sequence
    (:then_0
      (Utilities|FlowControl|DoOnce false
        (:Completed
          (bind _outactors (Actor|GetAllActorsOfClass "/Script/Engine.PlayerStart"))
          (bind _output_get_2 (Variables|Default|SetplayerStarts _outactors))
          (for _array_element _output_get_2
            (if (== (Variables|/Script/Engine.PlayerStart|GetPlayerStartTag _array_element) "Pink")
              (Utilities|Array|Add (Variables|Default|GetpinkPlayerStarts) _array_element)
              (else
                (Utilities|Array|Add (Variables|Default|GetgreenPlayerStarts) _array_element)))))))
    (:then_1
      (if (== (Variables|/Game/Lobby/PS_Lobby.PS_Lobby_C|GetPBDecalClass (.AsPS%20Lobby (Utilities|Casting|CastToPS_Lobby (Variables|/Script/Engine.Controller|GetPlayerState _output_get)))) "/Game/Blueprints/Decal/BP_DecalPink.BP_DecalPink_C")
        (CallFunction|SpawnActor (Variables|Default|GetpinkPlayerStarts))
        (else
          (CallFunction|SpawnActor (Variables|Default|GetgreenPlayerStarts)))))))

(fn ConstructionScript
  (|CallParentFunction))

(fn SpawnActor
  (params (playerStarts :type Array%20of%20Player%20Start%20Object%20References))
  ;[1 1 1] Spawn all actors
  (if (>= (Variables|Default|GetlastPlayerStart) (Utilities|Array|Length playerStarts))
    (Variables|Default|SetlastPlayerStart 0))
  (bind _returnvalue (Game|SpawnActorfromClass "/Game/ThirdPerson/Blueprints/BP_ThirdPersonCharacter.BP_ThirdPersonCharacter_C" (Transformation|GetActorTransform (Utilities|Array|Get(acopy) playerStarts (Variables|Default|GetlastPlayerStart))) "Undefined" "MultiplyWithRoot" (Variables|Default|GetnewPlayer) 0))
  (Math|Integer|IncrementInt (Variables|Default|GetlastPlayerStart)
    (:%20%20
      (Pawn|Possess (Variables|Default|GetnewPlayer) _returnvalue))))

(fn RespawnPlayer
  (params (playerStarts :type Array%20of%20Player%20Start%20Object%20References))
  (if (>= (Variables|Default|GetlastPlayerStart) (Utilities|Array|Length playerStarts))
    (Variables|Default|SetlastPlayerStart 0))
  (Transformation|SetActorTransform (Variables|Default|Getplayer%20to%20Respawn) (Transformation|GetActorTransform (Utilities|Array|Get(acopy) playerStarts (Variables|Default|GetlastPlayerStart))) false true)
  (Math|Integer|IncrementInt (Variables|Default|GetlastPlayerStart)))