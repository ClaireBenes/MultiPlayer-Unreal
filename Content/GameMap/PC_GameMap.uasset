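; Player controller for the multiplayer game map, handling each player's match flow from ready-up to end screen.
; On possession it disables pawn input and flags the player ready, with the IsReady RepNotify asking GS_GameMap to check all players.
; OC_ events drive countdown, input unlock with per-player score list, and end screen followed by servertravel to the lobby.
; Throw input, gated by CanPlay, spawns BP_Projectile through an S_ event.
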(event Custom|S_PlayerReady
  ;[1 1 1] Notify all ready player
  (Variables|Default|SetisReady true))

(event Custom|S_ThrowProjectile
  (bind _self self)
  ;[1 1 1] Throw projectile
  (Game|SpawnActorfromClass "/Game/Developers/clairebenes/Blueprint/BP_Projectile.BP_Projectile_C" (Transformation|GetWorldTransform (Variables|/Game/ThirdPerson/Blueprints/BP_ThirdPersonCharacter.BP_ThirdPersonCharacter_C|GetScene (.AsBP%20Third%20Person%20Character (Utilities|Casting|CastToBP_ThirdPersonCharacter (Pawn|GetControlledPawn))))) "Undefined" "MultiplyWithRoot" _self _self 0))

(event Custom|OC_DisableInput
  ;[1 1 1] Disable Input for 3 sec on start
  (Input|DisableInput (Pawn|GetControlledPawn) self)
  (CallFunction|SPlayerReady))

(event Custom|OC_ShowEndScreen
  (params (hasWon :type Boolean))
  ;[1 1 1] Show End Screen and travel back to lobby
  (bind _returnvalue (UserInterface|CreateWidget "/Game/Developers/clairebenes/Blueprint/Widget/WBP_EndScreen.WBP_EndScreen_C" self hasWon))
  (UserInterface|Viewport|AddtoViewport _returnvalue 0)
  (Input|DisableInput (Pawn|GetControlledPawn) self)
  (Utilities|FlowControl|Delay 0.5)
  (Development|ExecuteConsoleCommand "servertravel/Game/Developers/clairebenes/Map/LVL_Lobby" self))

(event Custom|OC_EnableInput
  ;[1 1 1] Enable Input
  (Input|EnableInput (Pawn|GetControlledPawn) self)
  ;;[0.3833 0.4599 1] Show Widget Score
  (bind _returnvalue (UserInterface|CreateWidget "/Game/Developers/clairebenes/Blueprint/Widget/WBP_Score.WBP_Score_C"))
  (bind _output_get (Variables|WBP|SetWBP%20Score _returnvalue))
  (UserInterface|Viewport|AddtoViewport _output_get 0)
  ;;[1 0.4129 0.2116] Show Name and Score of each player
  (for (_ _array_index) (Variables|/Script/Engine.GameStateBase|GetPlayerArray (Game|GetGameState))
    (bind _returnvalue_2 (UserInterface|CreateWidget "/Game/Developers/clairebenes/Blueprint/Widget/WBP_ScoreInfo.WBP_ScoreInfo_C" 0 _array_index))
    (Variables|/Script/UMG.TextBlock|SetText (Variables|/Game/Developers/clairebenes/Blueprint/Widget/WBP_ScoreInfo.WBP_ScoreInfo_C|GetTXT_Name _returnvalue_2) (Utilities|Text|ToText(Name) (Variables|/Game/Lobby/PS_Lobby.PS_Lobby_C|GetplayerTag (.AsPS%20Lobby (Utilities|Casting|CastToPS_Lobby (Game|GetPlayerState _array_index))))))
    (Widget|Panel|AddChild (Variables|/Game/Developers/clairebenes/Blueprint/Widget/WBP_Score.WBP_Score_C|GetVB_Score (Variables|WBP|GetWBP%20Score)) _returnvalue_2)
    (Variables|Default|SetcanPlay true)))

(event Custom|OC_StartCountdown
  ;[1 1 1] Show countdown widget on screen
  (bind _returnvalue (UserInterface|CreateWidget "/Game/Developers/clairebenes/Blueprint/Widget/WBP_Coutdown.WBP_Coutdown_C"))
  (bind _output_get (Variables|WBP|SetWBP%20Countdown _returnvalue))
  (UserInterface|Viewport|AddtoViewport _output_get 0))

(event Input|EnhancedActionEvents|EnhancedInputActionIA_Throw
  (params (ActionValue :type Boolean) (ElapsedSeconds :type Float%20%28double-precision%29) (TriggeredSeconds :type Float%20%28double-precision%29) (InputAction :type Input%20Action%20Object%20Reference :default "/Game/ThirdPerson/Input/Actions/IA_Throw.IA_Throw"))
  ;[1 1 1] Throw projectile
  (:Started
    (if (Variables|Default|GetcanPlay)
      (CallFunction|SThrowProjectile))))

(event EventBeginPlay
  ;[1 1 1] Begin Play
  (if (Pawn|IsLocalPlayerController)
    _))

(event EventPossess
  (params (PossessedPawn :type Pawn%20Object%20Reference))
  ;[1 1 1] On Possess
  (bind _asbp_third_person_character (Utilities|Casting|CastToBP_ThirdPersonCharacter PossessedPawn))
  (Default|OwnPossessed _asbp_third_person_character)
  (CallFunction|OCDisableInput))

(fn ConstructionScript)

(fn OnRepIsReady
  (bind _asgs_game_map (Utilities|Casting|CastToGS_GameMap (Game|GetGameState)))
  (Default|SCheckPlayersReady _asgs_game_map))