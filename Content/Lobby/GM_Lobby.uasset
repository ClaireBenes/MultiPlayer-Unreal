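; GM_Lobby is the lobby game mode that spawns and possesses a third-person character for each player who logs in.
; On PostLogin it saves through the game instance, then caches the PlayerStarts once and cycles through them round-robin for spawn transforms.
; Once the player count reaches the minimum, it reveals the Start Game button on the first player controller's lobby widget.
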(event EventPostLogin
  (params (NewPlayer :type Player%20Controller%20Object%20Reference))
  ;[1 1 1] Spawn character on login
  (Variables|Default|SetnewPlayer NewPlayer)
  (bind _asgi_framework (Utilities|Casting|CastToGI_Framework (Game|GetGameInstance)))
  (Default|SaveGame _asgi_framework)
  (Utilities|FlowControl|Sequence
    (:then_0
      (Utilities|FlowControl|DoOnce false
        (:Completed
          (bind _outactors (Actor|GetAllActorsOfClass "/Script/Engine.PlayerStart"))
          (Variables|Default|SetplayerStarts _outactors))))
    (:then_1
      (if (>= (Variables|Default|GetlastPlayerStart) (Utilities|Array|Length (Variables|Default|GetplayerStarts)))
        (Variables|Default|SetlastPlayerStart 0))
      (bind _returnvalue (Game|SpawnActorfromClass "/Game/ThirdPerson/Blueprints/BP_ThirdPersonCharacter.BP_ThirdPersonCharacter_C" (Transformation|GetActorTransform (Utilities|Array|Get(acopy) (Variables|Default|GetplayerStarts) (Variables|Default|GetlastPlayerStart))) "Undefined" "MultiplyWithRoot" (Variables|Default|GetnewPlayer) 0))
      (Math|Integer|IncrementInt (Variables|Default|GetlastPlayerStart)
        (:%20%20
          (Pawn|Possess (Variables|Default|GetnewPlayer) _returnvalue)
          (bind _aspc_lobby (Utilities|Casting|CastToPC_Lobby (Game|GetPlayerController 0)))
          (Utilities|IsValid _aspc_lobby
            (:Is%20Valid
              (bind _returnvalue_2 (Class|GameModeBase|GetNumPlayers))
              (if (>= _returnvalue_2 (Variables|Default|GetminNumberOfPlayer))
                (Widget|SetVisibility (Variables|/Game/Developers/clairebenes/Blueprint/Widget/WBP_SetPlayerInfo.WBP_SetPlayerInfo_C|GetB_StartGame (Variables|/Game/Lobby/PC_Lobby.PC_Lobby_C|GetWBP_SetPlayerInfo _aspc_lobby)) "Visible")))))))))

(fn ConstructionScript)