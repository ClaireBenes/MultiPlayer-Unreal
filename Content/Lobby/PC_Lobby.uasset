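; PC_Lobby is the lobby player controller, handling player info setup and projectile throwing.
; On BeginPlay, the local controller shows the WBP_SetPlayerInfo widget, and on possession it notifies the BP_ThirdPersonCharacter through OwnPossessed.
; Throw input waits briefly, then calls S_ThrowProjectile, which spawns a BP_Projectile at the character's ProjectileStart.
; The projectile receives the controller as owner and reference, plus the team color from PS_Lobby as its decal material.
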(event Custom|S_ThrowProjectile
  (bind _returnvalue (Pawn|GetControlledPawn))
  (bind _self self)
  (Game|SpawnActorfromClass "/Game/Developers/clairebenes/Blueprint/Projectile/BP_Projectile.BP_Projectile_C" (Transformation|GetWorldTransform (Variables|/Game/ThirdPerson/Blueprints/BP_ThirdPersonCharacter.BP_ThirdPersonCharacter_C|GetProjectileStart (.AsBP%20Third%20Person%20Character (Utilities|Casting|CastToBP_ThirdPersonCharacter _returnvalue)))) "Undefined" "MultiplyWithRoot" _self _self (Variables|/Game/Lobby/PS_Lobby.PS_Lobby_C|GetplayerTeamColor (.AsPS%20Lobby (Utilities|Casting|CastToPS_Lobby (Variables|/Script/Engine.Pawn|GetPlayerState _returnvalue)))) 0))

(event Input|EnhancedActionEvents|EnhancedInputActionIA_Throw
  (params (ActionValue :type Boolean) (ElapsedSeconds :type Float%20%28double-precision%29) (TriggeredSeconds :type Float%20%28double-precision%29) (InputAction :type Input%20Action%20Object%20Reference :default "/Game/ThirdPerson/Input/Actions/IA_Throw.IA_Throw"))
  (Utilities|FlowControl|Delay 0.2)
  (CallFunction|SThrowProjectile))

(event EventPossess
  (params (PossessedPawn :type Pawn%20Object%20Reference))
  (bind _asbp_third_person_character (Utilities|Casting|CastToBP_ThirdPersonCharacter PossessedPawn))
  (Default|OwnPossessed _asbp_third_person_character))

(event EventBeginPlay
  (if (Pawn|IsLocalPlayerController)
    (bind _returnvalue (UserInterface|CreateWidget "/Game/Developers/clairebenes/Blueprint/Widget/WBP_SetPlayerInfo.WBP_SetPlayerInfo_C"))
    (bind _output_get (Variables|Default|SetWBP_SetPlayerInfo _returnvalue))
    (UserInterface|Viewport|AddtoViewport _output_get 0)))

(fn ConstructionScript)